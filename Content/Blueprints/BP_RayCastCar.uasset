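; Player-drivable car Blueprint for a raycast-based vehicle, so far containing only the setup stage of the simulation.
; BeginPlay caches unit conversions and per-wheel components, then derives ray lengths, initial suspension lengths and wheel inertia from wheel and suspension data.
; It also sets front/rear torque ratios by drive type and brake ratios from bias.
; Tick only stores delta time, and the driving and gear input events are empty stubs.
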(event `self.ReceiveBeginPlay`
  ;[0.1156 0.3086 1] Event Begin to intialiase something first.
  (`self.Get Unit Convert Mul`)
  (`self.Store Component To Array`)
  (`self.RayCastINI`)
  (`self.SuspensionINI`)
  (`self.DriveTrainINI`)
  (`self.WheelINI`)
  (`self.BrakesINI`))

(event `self.ReceiveTick`
  (params (DeltaSeconds :type "Float (single-precision)"))
  (set `self.DeltaTime` DeltaSeconds))

(event `EnhancedInput|/Game/Inputs/Inputs/IA_Accelerate`
  (params (ActionValue :type "Float (double-precision)") (ElapsedSeconds :type "Float (double-precision)") (TriggeredSeconds :type "Float (double-precision)") (InputAction :type "InputAction Object Reference" :default "/Game/Inputs/Inputs/IA_Accelerate.IA_Accelerate")))

(event `EnhancedInput|/Game/Inputs/Inputs/IA_Brake`
  (params (ActionValue :type "Float (double-precision)") (ElapsedSeconds :type "Float (double-precision)") (TriggeredSeconds :type "Float (double-precision)") (InputAction :type "InputAction Object Reference" :default "/Game/Inputs/Inputs/IA_Brake.IA_Brake")))

(event `EnhancedInput|/Game/Inputs/Inputs/IA_Steer`
  (params (ActionValue :type "Float (double-precision)") (ElapsedSeconds :type "Float (double-precision)") (TriggeredSeconds :type "Float (double-precision)") (InputAction :type "InputAction Object Reference" :default "/Game/Inputs/Inputs/IA_Steer.IA_Steer")))

(event `Key|Tab`
  (params (Key :type "Key Structure")))

(event `EnhancedInput|/Game/Inputs/Inputs/IA_GearUp`
  (params (ActionValue :type Boolean) (ElapsedSeconds :type "Float (double-precision)") (TriggeredSeconds :type "Float (double-precision)") (InputAction :type "InputAction Object Reference" :default "/Game/Inputs/Inputs/IA_GearUp.IA_GearUp")))

(event `EnhancedInput|/Game/Inputs/Inputs/IA_GearDown`
  (params (ActionValue :type Boolean) (ElapsedSeconds :type "Float (double-precision)") (TriggeredSeconds :type "Float (double-precision)") (InputAction :type "InputAction Object Reference" :default "/Game/Inputs/Inputs/IA_GearDown.IA_GearDown")))

(fn `BrakesINI`
  (bind _returnvalue (`KismetMathLibrary.FClamp` (`self.BrakeBias`)))
  (set `self.BrakeRatio` (`|MakeArray` _returnvalue (- 1.0 _returnvalue))))

(fn `DriveTrainINI`
  (bind _drivetype (`self.DriveType`))
  (bind _returnvalue (`KismetMathLibrary.FClamp` (`self.TorqueBias`)))
  (if (== _drivetype 0)
    ;[1 1 1] FWD
    (set `self.TorqueRatio` (`|MakeArray` 1.0 0.0))
    (elif (== _drivetype 1)
      ;[1 1 1] RWD
      (set `self.TorqueRatio` (`|MakeArray` 0.0 1.0))
      (else
        ;[1 1 1] AWD
        (set `self.TorqueRatio` (`|MakeArray` _returnvalue (- _returnvalue 1.0)))))))

(fn `Get Unit Convert Mul`
  (bind _output_get (set `self.RPM_to_RadPS` (/ (* (`KismetMathLibrary.GetPI`) 2.0) 60.0)))
  (set `self.RadPS_to_RPM` (/ 1.0 _output_get)))

(fn `RayCastINI`
  (for _index (range 4)
    (bind (_rest_length _travel) (break `/Game/Structs_info/SuspensionStruct` (`|GetArrayItem` (`self.Suspension`) _index)))
    (`KismetArrayLibrary.Array_Set` (`self.RayLength`) _index (+ (`.radius_2_4B59FEFD4073B28AD32206B38321035E` (break `/Game/Structs_info/WheelStruct` (`|GetArrayItem` (`self.Wheel`) _index))) (+ _rest_length _travel)))))

(fn `Store Component To Array`
  (for _index (range 4)
    (`KismetArrayLibrary.Array_Set` (`self.TopLinkComponent`) _index (select `int` _index :`0` (`self.TopLink_FL`) :`1` (`self.TopLink_FR`) :`2` (`self.TopLink_RL`) :`3` (`self.TopLink_RR`)))
    (`KismetArrayLibrary.Array_Set` (`self.WheelComponent`) _index (select `int` _index :`0` (`self.Wheel_FL`) :`1` (`self.Wheel_FR`) :`2` (`self.Wheel_RL`) :`3` (`self.Wheel_RR`)))))

(fn `SuspensionINI`
  (for _index (range 4)
    (bind _rest_length (break `/Game/Structs_info/SuspensionStruct` (`|GetArrayItem` (`self.Suspension`) _index)))
    (`KismetArrayLibrary.Array_Set` (`self.Length`) _index _rest_length)
    (`KismetArrayLibrary.Array_Set` (`self.LastLength`) _index _rest_length)))

(fn `UserConstructionScript`)

(fn `WheelINI`
  (for _index (range 4)
    (bind (_radius _mass) (break `/Game/Structs_info/WheelStruct` (`|GetArrayItem` (`self.Wheel`) _index)))
    (`KismetArrayLibrary.Array_Set` (`self.WheelInertia`) _index (* (`KismetMathLibrary.MultiplyMultiply_FloatFloat` (/ _radius 100.0) 2.0) _mass 0.5))))